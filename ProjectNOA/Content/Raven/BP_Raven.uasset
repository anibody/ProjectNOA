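; Raven is an AI-controlled combat character that handles incoming attacks and switches reaction states through Blackboard flags on its Raven_Controller.
; Attacks are ignored while evading and counted while parrying, triggering a riposte at the required count; otherwise they drain HP and shield.
; Zero HP causes death, the first shield break causes stiffness, and an emptied groggy gauge causes groggy.
; State triggers, including knockdown and button action, first clear all flags through ResetState.
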(fn `beAttacked`
  (params (Damage :type "Float (double-precision)"))
  (bind _asraven_controller (cast `/Game/Raven/AI/Raven_Controller` (`self.GetController`)))
  (bind _blackboard (`AIController.Blackboard` _asraven_controller))
  (if (`BlackboardComponent.GetValueAsBool` _blackboard (`self.isEvading`))
    (`KismetSystemLibrary.PrintString` "공격 회피")
    (elif (`BlackboardComponent.GetValueAsBool` _blackboard (`self.isParrying`))
      (`self.Parrying`)
      (else
        (`self.getDamaged` Damage)))))

(fn `ButtonAction`
  (bind _asraven_controller (cast `/Game/Raven/AI/Raven_Controller` (`self.GetController`)))
  (bind _success (`self.resetState`))
  (if _success
    (`BlackboardComponent.SetValueAsBool` (`AIController.Blackboard` _asraven_controller) (`self.inButtonAction`) true)))

(fn `Die`
  (bind _asraven_controller (cast `/Game/Raven/AI/Raven_Controller` (`self.GetController`)))
  (bind _success (`self.resetState`))
  (if _success
    (`BlackboardComponent.SetValueAsBool` (`AIController.Blackboard` _asraven_controller) (`self.isDie`) true)))

(fn `getDamaged`
  (params (Damage :type "Float (double-precision)"))
  (if (> (`self.Hp`) 0.0)
    (bind _output_get (set `self.Hp` (- (`self.Hp`) Damage)))
    (if (> (`self.ShieldGauge`) 0.0)
      (bind _output_get_2 (set `self.ShieldGauge` (- (`self.ShieldGauge`) Damage))))
    (`KismetSystemLibrary.PrintString` (`KismetStringLibrary.Concat_StrStr` (`KismetStringLibrary.Concat_StrStr` "남은 체력 : " (`KismetStringLibrary.Conv_DoubleToString` _output_get)) (`KismetStringLibrary.Concat_StrStr` " 남은 실드 : " (`KismetStringLibrary.Conv_DoubleToString` _output_get_2))))
    (if (<= (`self.Hp`) 0.0)
      (`self.Die`)
      (elif (<= (`self.ShieldGauge`) 0.0)
        (if (not (`self.hasShieldBroken`))
          (set `self.hasShieldBroken` true)
          (`self.getStiffnessed`))))))

(fn `getGroggy`
  (if (> (`self.GroggyGauge`) 0)
    (bind _output_get (set `self.GroggyGauge` (- (`self.GroggyGauge`) 1)))
    (`KismetSystemLibrary.PrintString` (`KismetStringLibrary.Concat_StrStr` "남은 그로기 수치 : " (`KismetStringLibrary.Conv_IntToString` _output_get)))
    (if (<= (`self.GroggyGauge`) 0)
      (`self.Groggy`))))

(fn `getStiffnessed`
  (bind _asraven_controller (cast `/Game/Raven/AI/Raven_Controller` (`self.GetController`)))
  (bind _success (`self.resetState`))
  (if _success
    (`BlackboardComponent.SetValueAsBool` (`AIController.Blackboard` _asraven_controller) (`self.isStiffness`) true)))

(fn `Groggy`
  (bind _asraven_controller (cast `/Game/Raven/AI/Raven_Controller` (`self.GetController`)))
  (bind _success (`self.resetState`))
  (if _success
    (`BlackboardComponent.SetValueAsBool` (`AIController.Blackboard` _asraven_controller) (`self.isGroggy`) true)))

(fn `NockDown`
  (bind _asraven_controller (cast `/Game/Raven/AI/Raven_Controller` (`self.GetController`)))
  (bind _success (`self.resetState`))
  (if _success
    (`BlackboardComponent.SetValueAsBool` (`AIController.Blackboard` _asraven_controller) (`self.isNockDown`) true)))

(fn `Parrying`
  (bind _output_get (set `self.ParryingCount` (+ (`self.ParryingCount`) 1)))
  (`KismetSystemLibrary.PrintString` (`KismetStringLibrary.Concat_StrStr` "패링 친 횟수 : " (`KismetStringLibrary.Conv_ByteToString` _output_get)))
  (if (>= _output_get (`self.RequiredParryingCount`))
    (`self.ParryingRiposte`)))

(fn `ParryingRiposte`
  (bind _asraven_controller (cast `/Game/Raven/AI/Raven_Controller` (`self.GetController`)))
  (bind _success (`self.resetState`))
  (if _success
    (`BlackboardComponent.SetValueAsBool` (`AIController.Blackboard` _asraven_controller) (`self.isParryingRiposte`) true)))

(fn `recoverGroggyGauge`
  (set `self.GroggyGauge` (`self.MaximumGroggyGauge`)))

(fn `resetParryingCount`
  (set `self.ParryingCount` 0))

(fn `resetState`
  (returns (Success :type Boolean))
  (bind _asraven_controller (cast `/Game/Raven/AI/Raven_Controller` (`self.GetController`))
    (:`then`
      (bind _blackboard (`AIController.Blackboard` _asraven_controller))
      (`BlackboardComponent.SetValueAsBool` _blackboard (`self.isDie`) false)
      (`BlackboardComponent.SetValueAsBool` _blackboard (`self.isGroggy`) false)
      (`BlackboardComponent.SetValueAsBool` _blackboard (`self.isNockDown`) false)
      (`BlackboardComponent.SetValueAsBool` _blackboard (`self.isStiffness`) false)
      (`BlackboardComponent.SetValueAsBool` _blackboard (`self.inButtonAction`) false)
      (`BlackboardComponent.SetValueAsBool` _blackboard (`self.isEvading`) false)
      (`BlackboardComponent.SetValueAsBool` _blackboard (`self.isParrying`) false)
      (`self.resetParryingCount`)
      (`BlackboardComponent.SetValueAsBool` _blackboard (`self.isParryingRiposte`) false)
      (return true))
    (:`CastFailed`
      (return false))))

(fn `UserConstructionScript`)